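; Traffic light manager that cycles four lights from its TrafficLights array as two alternating pairs, starting on BeginPlay.
; Recolor sets one pair red and the other green, waits, switches all four to yellow, then waits briefly.
; It then calls itself with the lights in reverse order, swapping the pairs' roles in an endless Delay-driven loop.
; ChangeTrafficLightColor forwards the color enum to both lights of a pair.
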(event Custom|Recolor
  (params (TrafficLight :type BP%20Traffict%20Light%20Object%20Reference) (TrafficLight1 :type BP%20Traffict%20Light%20Object%20Reference) (TrafficLight2 :type BP%20Traffict%20Light%20Object%20Reference) (TrafficLight3 :type BP%20Traffict%20Light%20Object%20Reference))
  ;[1 1 1] Меняет цвет светофора на красный
  (CallFunction|ChangeTrafficLightColor TrafficLight TrafficLight1 "NewEnumerator0")
  ;[1 1 1] Меняет цвет светофора на зеленый
  (CallFunction|ChangeTrafficLightColor TrafficLight2 TrafficLight3 "NewEnumerator2")
  (Utilities|FlowControl|Delay 5.0)
  ;[1 1 1] Меняет цвет светофора на желтый
  (CallFunction|ChangeTrafficLightColor TrafficLight TrafficLight1 "NewEnumerator1")
  ;[1 1 1] Меняет цвет светофора на желтый
  (CallFunction|ChangeTrafficLightColor TrafficLight2 TrafficLight3 "NewEnumerator1")
  (Utilities|FlowControl|Delay 1.0)
  ;[1 1 1] Вызывает событие перекрашивания, но с обратным расположением светофоров
  (CallFunction|Recolor TrafficLight3 TrafficLight2 TrafficLight1 TrafficLight))

(event EventBeginPlay
  (bind _trafficlights (Variables|Default|GetTrafficLights))
  (CallFunction|Recolor (Utilities|Array|Get(acopy) _trafficlights) (Utilities|Array|Get(acopy) _trafficlights 1) (Utilities|Array|Get(acopy) _trafficlights 2) (Utilities|Array|Get(acopy) _trafficlights 3)))

(fn ConstructionScript)

(fn ChangeTrafficLightColor
  (params (TrafficLight :type BP%20Traffict%20Light%20Object%20Reference) (TrafficLight1 :type BP%20Traffict%20Light%20Object%20Reference) (Key :type E_LightColor%20Enum :default "NewEnumerator0"))
  (Default|ChangeColor TrafficLight Key)
  (Default|ChangeColor TrafficLight1 Key))